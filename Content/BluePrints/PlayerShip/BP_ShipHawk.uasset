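; Player ship Blueprint (Hawk) that the player steers by dragging a touch across the screen.
; While touched, Tick adds the touch delta, projected onto the ship's horizontal plane and scaled per axis, to a follow point the ship interpolates toward.
; Viewport corners deprojected onto that plane clamp the ship on screen at fixed height, while the spring arm follows sideways within limits.
; The G key toggles the mouse cursor and a GrabMode flag.
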(event `ClampMovement`
  (bind (_returnvalue_x _returnvalue_y) (`KismetMathLibrary.BreakVector` (`self.K2_GetActorLocation`)))
  (bind (_sizex _sizey) (`PlayerController.GetViewportSize` (`GameplayStatics.GetPlayerController` 0)))
  ;[0.05788 1 0.4489] Ограничение движения
  ;;[1 1 1] Создаем и проверяем худ
  (bind _output_get (set `self.HUD` (`PlayerController.GetHUD` (`GameplayStatics.GetPlayerController` 0))))
  (`/Engine/EditorBlueprintResources/StandardMacros.IsValid` _output_get
    (:`Is Valid`
      ;;[1 1 1] Присваиваем значение вьюпорта
      (set `self.SizeViewportX` (`KismetMathLibrary.Conv_IntToDouble` _sizex))
      (set `self.SizeViewportY` (`KismetMathLibrary.Conv_IntToDouble` _sizey))
      ;;[1 1 1] Начальные координаты угла вьюпорта
      (bind _output_get_2 (set `self.Angle00` (0.0 0.0)))
      (bind _output_get_3 (set `self.AngleXY` (`KismetMathLibrary.MakeVector2D` (`self.SizeViewportX`) (`self.SizeViewportY`))))
      (bind (_positionangle00_onplane _positionanglexy_onplane) (`self.GetPositionAnglesOnPlane` _output_get_2 _output_get_3))
      (bind (_x _y) (`KismetMathLibrary.BreakVector2D` _positionanglexy_onplane))
      (bind (_x_2 _y_2) (`KismetMathLibrary.BreakVector2D` _positionangle00_onplane))
      ;;[1 1 1] Присваиваем значения
      (`self.K2_SetActorLocation` (`KismetMathLibrary.MakeVector` (`KismetMathLibrary.FClamp` _returnvalue_x (+ _x 200.0) (- _x_2 200.0)) (`KismetMathLibrary.FClamp` _returnvalue_y (+ _y_2 100.0) (- _y 100.0)) 75.0)))))

(event `InputTouch`
  (params (Location :type "Vector Structure") (FingerIndex :type "ETouchIndex Enum"))
  (bind (_locationx _locationy) (`PlayerController.GetInputTouchState` (`GameplayStatics.GetPlayerController` 0) "Touch1"))
  ;[1 0 0.1114] Рассчет перемещения корабля
  (:`Pressed`
    (set `self.IsPresssed` true)
    ;;[1 1 1] Получаем значение корабля
    (set `self.ShipFollowPoint` (`self.K2_GetActorLocation`))
    ;;[1 1 1] Презаписываем начальные координаты
    (set `self.LastTouchPosition` (`KismetMathLibrary.MakeVector2D` _locationx _locationy)))
  (:`Released`
    (set `self.IsPresssed` false)))

(event `CoridinateCurret`
  (bind (_lasttouchposition_x _lasttouchposition_y) (`KismetMathLibrary.BreakVector2D` (`self.LastTouchPosition`)))
  (bind (_currentinrersecton_x _currentinrersecton_y) (`KismetMathLibrary.BreakVector2D` (`self.GetTouchPosistionShipPlane` (`KismetMathLibrary.MakeVector2D` _lasttouchposition_x _lasttouchposition_y))))
  (bind (_locationx _locationy) (`PlayerController.GetInputTouchState` (`GameplayStatics.GetPlayerController` 0) "Touch1"))
  (bind (_currentinrersecton_x_2 _currentinrersecton_y_2) (`KismetMathLibrary.BreakVector2D` (`self.GetTouchPosistionShipPlane` (`KismetMathLibrary.MakeVector2D` _locationx _locationy))))
  (bind (_returnvalue_x _returnvalue_y) (`KismetMathLibrary.BreakVector` (- (`KismetMathLibrary.MakeVector` _currentinrersecton_x_2 _currentinrersecton_y_2) (`KismetMathLibrary.MakeVector` _currentinrersecton_x _currentinrersecton_y))))
  ;[1 0 0.1114] Рассчет перемещения корабля
  ;;[1 1 1] Прибавляем координаты точки к координатам корабля
  (set `self.ShipFollowPoint` (+ (`self.ShipFollowPoint`) (`KismetMathLibrary.MakeVector` (* _returnvalue_x (`self.MoveSpeedX`)) (* _returnvalue_y (`self.MoveSpeedY`)))))
  ;;[1 1 1] Перезаписываем на конечное положение
  (set `self.LastTouchPosition` (`KismetMathLibrary.MakeVector2D` _locationx _locationy)))

(event `Key|G`
  (params (Key :type "Key Structure"))
  (bind _returnvalue (`GameplayStatics.GetPlayerController` 0))
  ;[0 0.25 1] Включаем или выключам курсор
  (:`Pressed`
    (set `self.GrabMode` (not (`self.GrabMode`)))
    (set `PlayerController.bShowMouseCursor` (not (`PlayerController.bShowMouseCursor` _returnvalue)) _returnvalue)))

(event `CameraRotation`
  (bind (_returnvalue_x _returnvalue_y) (`KismetMathLibrary.BreakVector` (`SceneComponent.K2_GetComponentLocation` (`self.BodyMesh`))))
  ;[1 0.2199 0.9465] Перемещение камеры
  (`SceneComponent.K2_SetWorldLocation` (`self.SpringArm`) (`KismetMathLibrary.MakeVector` 0.0 (`KismetMathLibrary.FClamp` _returnvalue_y -800.0 800.0)) false false))

(event `self.ReceiveTick`
  (params (DeltaSeconds :type "Float (single-precision)"))
  (if (`self.IsPresssed`)
    (`self.CameraRotation`)
    (`self.CoridinateCurret`)
    ;[1 1 1] Присваивае значение интерполяции к знаяение корабля
    (`self.K2_SetActorLocation` (`KismetMathLibrary.VInterpTo` (`self.K2_GetActorLocation`) (`self.ShipFollowPoint`) DeltaSeconds 30.0))
    ;[1 1 1] Ограничение движения
    (`self.ClampMovement`)))

(fn `GetPositionAnglesOnPlane`
  (params (Angle00 :type "Vector2D Structure") (AngleXY :type "Vector2D Structure"))
  (returns (`PositionAngle00 OnPlane` :type "Vector2D Structure") (`PositionAngleXY OnPlane` :type "Vector2D Structure"))
  (bind _returnvalue (`GameplayStatics.GetPlayerController` 0))
  (bind _returnvalue_2 (`PlayerCameraManager.GetCameraLocation` (`PlayerController.PlayerCameraManager` _returnvalue)))
  (bind _returnvalue_3 (`PlayerCameraManager.GetCameraLocation` (`PlayerController.PlayerCameraManager` _returnvalue)))
  (bind (_t _intersection) (`KismetMathLibrary.LinePlaneIntersection` _returnvalue_2 (+ _returnvalue_2 (* (`.WorldDirection` (`PlayerController.DeprojectScreenPositionToWorld` _returnvalue AngleXY_X AngleXY_Y)) 10000.0)) (`KismetMathLibrary.MakePlaneFromPointAndNormal` (`self.K2_GetActorLocation`) (0.0 0.0 1.0))))
  (bind (_t_2 _intersection_2) (`KismetMathLibrary.LinePlaneIntersection` _returnvalue_3 (+ _returnvalue_3 (* (`.WorldDirection` (`PlayerController.DeprojectScreenPositionToWorld` _returnvalue Angle00_X Angle00_Y)) 10000.0)) (`KismetMathLibrary.MakePlaneFromPointAndNormal` (`self.K2_GetActorLocation`) (0.0 0.0 1.0))))
  (return (`KismetMathLibrary.MakeVector2D` (.x _intersection_2) (.y _intersection_2)) (`KismetMathLibrary.MakeVector2D` (.x _intersection) (.y _intersection))))

(fn `GetTouchPosistionShipPlane`
  (params (Position :type "Vector2D Structure"))
  (returns (CurrentInrersecton :type "Vector2D Structure"))
  (bind _returnvalue (`GameplayStatics.GetPlayerController` 0))
  (bind _returnvalue_2 (`PlayerCameraManager.GetCameraLocation` (`PlayerController.PlayerCameraManager` _returnvalue)))
  (bind (_t _intersection) (`KismetMathLibrary.LinePlaneIntersection` _returnvalue_2 (+ _returnvalue_2 (* (`.WorldDirection` (`PlayerController.DeprojectScreenPositionToWorld` _returnvalue Position_X Position_Y)) 10000.0)) (`KismetMathLibrary.MakePlaneFromPointAndNormal` (`self.K2_GetActorLocation`) (0.0 0.0 1.0))))
  (return (`KismetMathLibrary.MakeVector2D` (.x _intersection) (.y _intersection))))

(fn `UserConstructionScript`)