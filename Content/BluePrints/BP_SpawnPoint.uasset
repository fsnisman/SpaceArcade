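; Spawn point actor that tracks when the player ship's enemy death count reaches the total needed to flag a boss spawn.
; At BeginPlay it finds BP_ShipHawk and sums CountEnemy across all spawn points tagged "Enemy".
; Tick compares that total with the ship's CountDiedEnemyPawn, then sets SpawnBoss once and decrements the total.
; The graph only sets the flag and contains no spawning logic.
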(event `self.ReceiveBeginPlay`
  (bind _returnvalue (`GameplayStatics.GetActorOfClass` "/Game/BluePrints/PlayerShip/BP_ShipHawk.BP_ShipHawk_C"))
  (set `self.PlayerShip` _returnvalue)
  (bind _outactors (`GameplayStatics.GetAllActorsOfClassWithTag` "BP_SpawnPoint_C" "Enemy"))
  (for _array_element _outactors
    (bind _output_get (set `self.SpawnPoint` _array_element))
    (set `self.Array Enemy Pawn` (+ (`SpawnEnymyShip.CountEnemy` _output_get) (`self.Array Enemy Pawn`)))))

(event `self.ReceiveTick`
  (params (DeltaSeconds :type "Float (single-precision)"))
  (bind _playership (`self.PlayerShip`))
  (`/Engine/EditorBlueprintResources/StandardMacros.IsValid` _playership
    (:`Is Valid`
      (if (`self.SpawnBoss`)
        _
        (elif (== (`PlayerShipPawn.CountDiedEnemyPawn` _playership) (`self.Array Enemy Pawn`))
          (set `self.SpawnBoss` true)
          (`/Engine/EditorBlueprintResources/StandardMacros.DecrementFloat` (`self.Array Enemy Pawn`)))))))

(fn `UserConstructionScript`)