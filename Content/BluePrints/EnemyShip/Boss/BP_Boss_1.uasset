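; Boss enemy ship Blueprint that moves along Y after a startup delay and plays a scripted movement when killed.
; The Move timeline offsets BodyMesh each update until HealthComponent health reaches zero.
; Tick polls health, then on death disables hit collider and mesh collision and plays parallel timelines for downward, forward and yaw motion.
; Timeline_1 is unconnected and never runs.
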(event `self.ReceiveBeginPlay`
  (`KismetSystemLibrary.Delay` 8.0)
  (bind (_direction _move) (`Timeline|Move` :!via `PlayFromStart` :!label _label)
    (:`Update`
      (if (<= (`HealthComponent.CurrentHealth` (`self.HealthComponent`)) 0.0)
        (goto _label :!via `Stop`)
        (else
          (`SceneComponent.K2_AddWorldOffset` (`self.BodyMesh`) (`KismetMathLibrary.MakeVector` 0.0 _move) false false))))))

(event `self.ReceiveTick`
  (params (DeltaSeconds :type "Float (single-precision)"))
  (if (<= (`HealthComponent.CurrentHealth` (`self.HealthComponent`)) 0.0)
    (`PrimitiveComponent.SetCollisionEnabled` (`self.HitCollider`) "NoCollision")
    (`PrimitiveComponent.SetCollisionEnabled` (`self.HitCollider3`) "NoCollision")
    (`PrimitiveComponent.SetCollisionEnabled` (`self.HitCollider2`) "NoCollision")
    (`PrimitiveComponent.SetCollisionEnabled` (`self.BodyMesh`) "NoCollision")
    (`|ExecutionSequence`
      (:`then_0`
        (bind (_direction _move) (`Timeline|Move Down`)
          (:`Update`
            (`SceneComponent.K2_AddWorldOffset` (`self.BodyMesh`) (`KismetMathLibrary.MakeVector` 0.0 0.0 _move) false false))))
      (:`then_1`
        (bind (_direction_2 _move_2) (`Timeline|Move Forward`)
          (:`Update`
            (`SceneComponent.K2_AddWorldOffset` (`self.BodyMesh`) (`KismetMathLibrary.MakeVector` _move_2) false false))))
      (:`then_2`
        (bind (_direction_3 _move_3) (`Timeline|Rotate`)
          (:`Update`
            (`SceneComponent.K2_AddRelativeRotation` (`self.BodyMesh`) (`KismetMathLibrary.MakeRotator` 0.0 0.0 _move_3) false false)))))))

(fn `UserConstructionScript`)