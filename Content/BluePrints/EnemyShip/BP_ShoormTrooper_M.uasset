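; BP_ShoormTrooper_M is an enemy pawn that makes a delayed, scripted move and reports its removal to the player's ShipHawk.
; On BeginPlay it caches the ship, waits, then a timeline offsets BodyMesh along X.
; When that timeline finishes, it destroys itself and increments the ship's CountDiedEnemyPawn, regardless of damage.
; HealthComponent damage restarts a second timeline driving the "Switch" material parameter as hit feedback.
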(event `self.ReceiveBeginPlay`
  (bind _returnvalue (`GameplayStatics.GetActorOfClass` "/Game/BluePrints/PlayerShip/BP_ShipHawk.BP_ShipHawk_C"))
  (set `self.PlayerShip` _returnvalue)
  (`KismetSystemLibrary.Delay` 8.0)
  (bind (_direction _move) (`Timeline|Timeline_0`)
    (:`Update`
      (`SceneComponent.K2_AddWorldOffset` (`self.BodyMesh`) (`KismetMathLibrary.MakeVector` _move) false false))
    (:`Finished`
      (`self.K2_DestroyActor`)
      (`/Engine/EditorBlueprintResources/StandardMacros.IncrementFloat` (`PlayerShipPawn.CountDiedEnemyPawn` (`self.PlayerShip`))))))

(event `self.HealthComponent.OnDamaged`
  (params (DamageValue :type "Float (single-precision)"))
  (bind (_direction _switch) (`Timeline|Timeline_1` :!via `PlayFromStart`)
    (:`Update`
      (`MeshComponent.SetScalarParameterValueOnMaterials` (`self.BodyMesh`) "Switch" _switch))))

(fn `UserConstructionScript`)