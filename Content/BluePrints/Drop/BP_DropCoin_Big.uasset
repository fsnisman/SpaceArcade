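; BP_DropCoin_Big is a large coin drop actor that spins while moving along the world X axis.
; BeginPlay sets the mesh's starting rotation and plays the Down timeline, whose track supplies a per-update offset for BodyMesh.
; Each update reads the Pause flag from GameHud and applies a zero offset while paused.
; Tick adds roll by the Rotate variable every frame, regardless of pause or delta time.
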(event `self.ReceiveBeginPlay`
  ;[1 1 1] Вращение объекта
  (`SceneComponent.K2_SetWorldRotation` (`self.BodyMesh`) (struct :`Pitch` 90.0 :`Roll` -60.0) false false)
  (bind (_direction _newtrack_0) (`Timeline|Down`)
    (:`Update`
      ;;[1 1 1] Проверка на паузу
      (bind _asgame_hud (cast `GameHud` (`PlayerController.GetHUD` (`GameplayStatics.GetPlayerController` 0))))
      (if (`GameHud.bPause` _asgame_hud)
        (`SceneComponent.K2_AddWorldOffset` (`self.BodyMesh`) (0.0 0.0 0.0) false false)
        (else
          (`SceneComponent.K2_AddWorldOffset` (`self.BodyMesh`) (`KismetMathLibrary.MakeVector` _newtrack_0) false false))))))

(event `self.ReceiveTick`
  (params (DeltaSeconds :type "Float (single-precision)"))
  ;[1 1 1] Перемещение вниз
  (`SceneComponent.K2_AddWorldRotation` (`self.BodyMesh`) (`KismetMathLibrary.MakeRotator` (`self.Rotate`)) false false))

(fn `UserConstructionScript`)