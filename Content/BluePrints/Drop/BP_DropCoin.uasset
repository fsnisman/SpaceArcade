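; BP_DropCoin is a dropped coin actor that spins while a timeline moves it.
; On BeginPlay it tilts BodyMesh and plays the Down timeline, whose track feeds a world X offset on each update.
; While the GameHud Pause flag is set, that offset is zero, though the timeline keeps playing.
; Tick adds a roll rotation every frame regardless of pause, and no pickup logic is present.
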(event `self.ReceiveBeginPlay`
  (`SceneComponent.K2_SetWorldRotation` (`self.BodyMesh`) (struct :`Pitch` 90.0 :`Roll` -60.0) false false)
  (bind (_direction _newtrack_0) (`Timeline|Down`)
    (:`Update`
      (bind _asgame_hud (cast `GameHud` (`PlayerController.GetHUD` (`GameplayStatics.GetPlayerController` 0))))
      (if (`GameHud.bPause` _asgame_hud)
        (`SceneComponent.K2_AddWorldOffset` (`self.BodyMesh`) (0.0 0.0 0.0) false false)
        (else
          (`SceneComponent.K2_AddWorldOffset` (`self.BodyMesh`) (`KismetMathLibrary.MakeVector` _newtrack_0) false false))))))

(event `self.ReceiveTick`
  (params (DeltaSeconds :type "Float (single-precision)"))
  (`SceneComponent.K2_AddWorldRotation` (`self.BodyMesh`) (`KismetMathLibrary.MakeRotator` (`self.Rotate`)) false false))

(fn `UserConstructionScript`)